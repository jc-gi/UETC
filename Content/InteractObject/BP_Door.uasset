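; BP_Door is an interactable door that the player toggles with the E key while standing near it.
; Box overlap with BP_Character enables input and shows an IntInteraction prompt widget, and leaving reverses both.
; A FlipFlop on E alternately plays and reverses the Abrir_Puerta timeline, but no graph logic applies its output to the door, as the open/close Lerp is unconnected.
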(event `Key|E`
  (params (Key :type "Key Structure"))
  ;[1 1 1] qUE PASA CUANDO SE PRESIONA E
  (:`Pressed`
    (`/Engine/EditorBlueprintResources/StandardMacros.FlipFlop`
      (:`A`
        (bind (_direction _animdoor) (`Timeline|Abrir_Puerta` :!label _label)))
      (:`B`
        (goto _label :!via `Reverse`)))))

(event `self.Box.OnComponentBeginOverlap`
  (params (OverlappedComponent :type "PrimitiveComponent Object Reference") (OtherActor :type "Actor Object Reference") (OtherComp :type "PrimitiveComponent Object Reference") (OtherBodyIndex :type Integer) (bFromSweep :type Boolean) (SweepResult :type "HitResult Structure (by ref)"))
  ;[1 1 1] Detecta la colision
  ;[1 1 1] Colision Personaje
  (cast `/Game/Character/Blueprints/BP_Character` OtherActor)
  (`self.EnableInput` (`GameplayStatics.GetPlayerController` 0))
  ;[1 1 1] Muestra Interfaz
  (bind _returnvalue (`|CreateWidget` "/Game/Interfaces/IntInteraction.IntInteraction_C"))
  (`UserWidget.AddToViewport` _returnvalue 0))

(event `self.Box.OnComponentEndOverlap`
  (params (OverlappedComponent :type "PrimitiveComponent Object Reference") (OtherActor :type "Actor Object Reference") (OtherComp :type "PrimitiveComponent Object Reference") (OtherBodyIndex :type Integer))
  ;[1 1 1] Desactiva Colision
  (cast `/Game/Character/Blueprints/BP_Character` OtherActor)
  (`self.DisableInput` (`GameplayStatics.GetPlayerController` 0))
  (`Widget.RemoveFromParent` (stale `self.Box.OnComponentBeginOverlap` _returnvalue)))

(fn `UserConstructionScript`)